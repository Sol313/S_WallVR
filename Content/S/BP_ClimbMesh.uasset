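; BP_ClimbMesh is a climbable object that lets the motion controller pawn pull itself along by hand.
; Climb and Fall track up to two gripping controllers, update the pawn's ClimbingHands count, and re-anchor the pivot to the newest or remaining hand.
; While the pawn is climbing, Tick offsets it by the active controller's drift from that pivot, then snaps the controller back onto the pivot.
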(event EventTick
  (params (DeltaSeconds :type Float%20%28single-precision%29))
  (bind _firstmc (Variables|Default|GetFirstMC))
  (bind _secondmc (Variables|Default|GetSecondMC))
  (bind _secondmc_2 (Variables|Default|GetSecondMC))
  (bind _returnvalue (Utilities|IsValid _secondmc_2))
  (bind _returnvalue_2 (select _returnvalue _secondmc _firstmc))
  (if (Utilities|IsValid (Variables|Default|GetMCPawn))
    (if (and (Variables|/Game/VirtualRealityBP/Blueprints/MotionControllerPawn.MotionControllerPawn_C|GetIsClimbing (Variables|Default|GetMCPawn)) (Utilities|IsValid (Variables|Default|GetFirstMC)))
      (Transformation|AddActorWorldOffset (Variables|Default|GetMCPawn) (- (Variables|Default|GetPivotPoint) (Transformation|GetWorldLocation _returnvalue_2)))
      (Transformation|SetWorldLocation _returnvalue_2 (Variables|Default|GetPivotPoint) false false))))

(event EventClimb
  (params (MotionController :type Scene%20Component%20Object%20Reference))
  (if (Utilities|IsValid (Variables|Default|GetFirstMC))
    (Variables|Default|SetSecondMC MotionController)
    (else
      (Variables|Default|SetFirstMC MotionController)))
  (Variables|Default|SetPivotPoint (Transformation|GetWorldLocation (select (Utilities|IsValid (Variables|Default|GetSecondMC)) (Variables|Default|GetSecondMC) (Variables|Default|GetFirstMC))))
  (bind _asmotion_controller_pawn (Utilities|Casting|CastToMotionControllerPawn (Game|Player|GetPlayerPawn 0)))
  (bind _output_get (Variables|Default|SetMCPawn _asmotion_controller_pawn))
  (Math|Integer|IncrementInt (Variables|/Game/VirtualRealityBP/Blueprints/MotionControllerPawn.MotionControllerPawn_C|GetClimbingHands _output_get)))

(event EventFall
  (params (MotionController :type Scene%20Component%20Object%20Reference))
  (if (Utilities|IsValid (Variables|Default|GetSecondMC))
    (if (== MotionController (Variables|Default|GetSecondMC))
      (Variables|Default|SetSecondMC 0)
      (Variables|Default|SetPivotPoint (Transformation|GetWorldLocation (Variables|Default|GetFirstMC)))
      (else
        (Variables|Default|SetFirstMC (Variables|Default|GetSecondMC))
        (Variables|Default|SetSecondMC 0)
        (Variables|Default|SetPivotPoint (Transformation|GetWorldLocation (Variables|Default|GetFirstMC)))))
    (Math|Integer|DecrementInt (Variables|/Game/VirtualRealityBP/Blueprints/MotionControllerPawn.MotionControllerPawn_C|GetClimbingHands (Variables|Default|GetMCPawn)) :!label _label)
    (elif (== MotionController (Variables|Default|GetFirstMC))
      (Variables|Default|SetFirstMC 0)
      (Variables|Default|SetSecondMC 0)
      (Variables|Default|SetPivotPoint "0, 0, 0")
      (goto _label))))

(fn ConstructionScript)